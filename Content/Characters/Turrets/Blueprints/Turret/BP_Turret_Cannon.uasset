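; BP_Turret_Cannon is a cannon turret that targets BP_Paladin characters and fires cannonballs at them.
; Its Sphere overlap stores the first Paladin to enter as the current target while none is valid, with no end-overlap release.
; While the target is valid and CanShoot is true, Tick turns the whole actor toward it.
; A Delay on Tick paces BP_CannonBall spawns at the Arrow's transform to roughly every 2.5 seconds.
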(event `self.ReceiveTick`
  (params (DeltaSeconds :type "Float (single-precision)"))
  (if (`KismetSystemLibrary.IsValid` (`self.CurrentTarget`))
    (if (`self.CanShoot`)
      (`self.K2_SetActorRotation` (`KismetMathLibrary.FindLookAtRotation` (`self.K2_GetActorLocation`) (`self.K2_GetActorLocation` (`self.CurrentTarget`))))
      (`KismetSystemLibrary.Delay` 2.5)
      (`|SpawnActorFromClass` "/Game/Characters/Turrets/Blueprints/Projectiles/BP_CannonBall.BP_CannonBall_C" (`SceneComponent.K2_GetComponentToWorld` (`self.Arrow`)) "Undefined" "OverrideRootScale" null null))))

(event `self.Sphere.OnComponentBeginOverlap`
  (params (OverlappedComponent :type "PrimitiveComponent Object Reference") (OtherActor :type "Actor Object Reference") (OtherComp :type "PrimitiveComponent Object Reference") (OtherBodyIndex :type Integer) (bFromSweep :type Boolean) (SweepResult :type "HitResult Structure (by ref)"))
  (if (not (`KismetSystemLibrary.IsValid` (`self.CurrentTarget`)))
    (bind _asbp_paladin (cast `/Game/NPC/BP/BP_Paladin` OtherActor))
    (set `self.CurrentTarget` _asbp_paladin)))

(fn `UserConstructionScript`)