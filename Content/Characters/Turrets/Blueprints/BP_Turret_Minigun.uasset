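; Minigun turret that locks onto a BP_Paladin it sees and fires BP_Bullet actors at it.
; PawnSensing sightings drive everything: with no valid target, a seen Paladin becomes CurrentTarget.
; Later sightings of any pawn turn the whole actor toward that target, then spawn a bullet at the Arrow component after a short Delay.
; The target is kept until it becomes invalid.
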(event `self.PawnSensing.OnSeePawn`
  (params (Pawn :type "Pawn Object Reference"))
  (if (`KismetSystemLibrary.IsValid` (`self.CurrentTarget`))
    (`self.K2_SetActorRotation` (`KismetMathLibrary.FindLookAtRotation` (`self.K2_GetActorLocation`) (`self.K2_GetActorLocation` (`self.CurrentTarget`))))
    (`KismetSystemLibrary.Delay` 0.2)
    (`|SpawnActorFromClass` "/Game/Characters/Turrets/Blueprints/BP_Bullet.BP_Bullet_C" (`SceneComponent.K2_GetComponentToWorld` (`self.Arrow`)) "Undefined" "OverrideRootScale" null null)
    (else
      (bind _asbp_paladin (cast `/Game/NPC/BP/BP_Paladin` Pawn))
      (set `self.CurrentTarget` _asbp_paladin))))

(fn `UserConstructionScript`)