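; BP_IceBall is the wizard character's ice projectile actor, which freezes and damages goblins it hits.
; A sphere overlap that casts to BPC_Goblin sets its Freeze flag, applies damage, spawns an explosion emitter with a sound, then destroys the ball after a tiny delay.
; Anything other than a goblin is ignored, and the ball destroys itself after a five-second lifetime.
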(event `self.ReceiveBeginPlay`
  (`KismetSystemLibrary.Delay` 5.0)
  (`self.K2_DestroyActor`))

(event `self.Sphere.OnComponentBeginOverlap`
  (params (OverlappedComponent :type "PrimitiveComponent Object Reference") (OtherActor :type "Actor Object Reference") (OtherComp :type "PrimitiveComponent Object Reference") (OtherBodyIndex :type Integer) (bFromSweep :type Boolean) (SweepResult :type "HitResult Structure (by ref)"))
  (bind _asbpc_goblin (cast `/Game/NPC/BP/BPC_Goblin` OtherActor))
  (set `/Game/NPC/BP/BPC_Goblin.Freeze` true _asbpc_goblin)
  (`GameplayStatics.ApplyDamage` OtherActor 20.0)
  (`GameplayStatics.SpawnEmitterAtLocation` "/Game/StarterContent/Particles/P_Explosion.P_Explosion" (`SceneComponent.K2_GetComponentLocation` (`self.Sphere`)))
  (`GameplayStatics.PlaySound2D` "/Game/StarterContent/Audio/Collapse01.Collapse01" 0.3 1.0 0.0 null null)
  (`KismetSystemLibrary.Delay` 0.01)
  (`self.K2_DestroyActor`))

(fn `UserConstructionScript`)