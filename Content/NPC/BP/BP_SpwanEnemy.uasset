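; Spawner actor that creates BP_Paladin AI pawns at its own location, starting with one on BeginPlay.
; The RevisarEnemys event compares CurrentAmount to MaxAmount and, while they differ, increments the count and spawns another Paladin after a short delay.
; At the maximum it only runs a longer delay with nothing after it.
; Nothing in this Blueprint calls RevisarEnemys or decrements the count.
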(event `self.ReceiveBeginPlay`
  (`self.Spawn Enemy`))

(event `RevisarEnemys`
  (if (== (`self.currentAmount`) (`self.MaxAmount`))
    (`KismetSystemLibrary.Delay` 30.0)
    (else
      (set `self.currentAmount` (+ (`self.currentAmount`) 1))
      (`KismetSystemLibrary.Delay` 2.0)
      (`self.Spawn Enemy`))))

(event `Spawn Enemy`
  (`AIBlueprintHelperLibrary.SpawnAIFromClass` "/Game/NPC/BP/BP_Paladin.BP_Paladin_C" null (`self.K2_GetActorLocation`) (struct) false null))

(fn `UserConstructionScript`)