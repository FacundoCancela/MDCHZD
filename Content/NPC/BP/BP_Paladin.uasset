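; Paladin enemy NPC that chases and attacks the wizard player, registering in the game mode's alive count.
; Box overlap starts a looping attack of shuffled montage sections and damage; GotoPlayer drives AI movement.
; Tick updates a player-facing health bar and polls elemental status flags, using delays for damage, movement freezes and resets.
; Lethal damage disables collision, plays a death animation, decrements the count and destroys the actor.
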(event `self.ReceiveBeginPlay`
  (bind _asbp_third_person_game_mode (cast `/Game/ThirdPerson/Blueprints/BP_ThirdPersonGameMode` (`GameplayStatics.GetGameMode`)))
  (set `/Game/ThirdPerson/Blueprints/BP_ThirdPersonGameMode.PaldinAlives` (+ (`/Game/ThirdPerson/Blueprints/BP_ThirdPersonGameMode.PaldinAlives` _asbp_third_person_game_mode) 1) _asbp_third_person_game_mode))

(event `self.Box.OnComponentEndOverlap`
  (params (OverlappedComponent :type "PrimitiveComponent Object Reference") (OtherActor :type "Actor Object Reference") (OtherComp :type "PrimitiveComponent Object Reference") (OtherBodyIndex :type Integer))
  (cast `/Game/Characters/WizzardCharacter/BPCharacter_Wizard` OtherActor)
  (set `self.Attacking` false))

(event `self.Box.OnComponentBeginOverlap`
  (params (OverlappedComponent :type "PrimitiveComponent Object Reference") (OtherActor :type "Actor Object Reference") (OtherComp :type "PrimitiveComponent Object Reference") (OtherBodyIndex :type Integer) (bFromSweep :type Boolean) (SweepResult :type "HitResult Structure (by ref)"))
  (cast `/Game/Characters/WizzardCharacter/BPCharacter_Wizard` OtherActor)
  (set `self.Attacking` true)
  (`self.Attack Player`))

(event `Attack Player`
  ;[1 1 1] Atacar Player
  (`KismetArrayLibrary.Array_Shuffle` (`self.Secciones`))
  (bind _returnvalue (`self.PlayAnimMontage` "/Game/NPC/Animations/AM_Paladin.AM_Paladin" 1.0 (`|GetArrayItem` (`self.Secciones`))))
  (`KismetSystemLibrary.Delay` _returnvalue)
  (`GameplayStatics.ApplyDamage` (stale `self.Box.OnComponentBeginOverlap` OtherActor) 15.0)
  (if (`self.Attacking`)
    (`self.Attack Player`)))

(event `self.ReceiveTick`
  (params (DeltaSeconds :type "Float (single-precision)"))
  (`|ExecutionSequence`
    (:`then_0`
      (bind _aswbp_enemy_life (cast `/Game/Widgets/Wenemy/WBP_EnemyLife` (`WidgetComponent.GetUserWidgetObject` (`self.Widget`))))
      (`ProgressBar.SetPercent` (`/Game/Widgets/Wenemy/WBP_EnemyLife.LifeBar` _aswbp_enemy_life) (/ (`self.Health`) 100.0))
      (`SceneComponent.K2_SetWorldRotation` (`self.Widget`) (`KismetMathLibrary.MakeRotator` 0.0 0.0 (.yaw (`KismetMathLibrary.FindLookAtRotation` (`SceneComponent.K2_GetComponentLocation` (`self.Widget`)) (`self.K2_GetActorLocation` (`GameplayStatics.GetPlayerCharacter` 0))))) false false)
      (if (<= (`self.Health`) 0.0)
        (`/Engine/EditorBlueprintResources/StandardMacros.DoOnce` false
          (:`Completed`
            (`PrimitiveComponent.SetSimulatePhysics` (`self.Widget`) true)
            (if (`self.isDead`)
              (`self.K2_DestroyActor`)
              (set `self.isDead` true))))))
    (:`then_1`
      (`|ExecutionSequence`
        (:`then_0`
          (if (`self.Burn`)
            (`KismetSystemLibrary.Delay` 3.0)
            (set `self.Health` (- (`self.Health`) 5.0))))
        (:`then_1`
          (if (`self.Burn`)
            (`KismetSystemLibrary.Delay` 2.0)
            (set `self.Burn` false)))))
    (:`then_2`
      (if (`self.Freeze`)
        (`GameplayStatics.SpawnEmitterAtLocation` "/Game/InfinityBladeEffects/Effects/FX_Monsters/FX_Monster_FrostGiant/ICE/P_ArmBuildUp01.P_ArmBuildUp01" (`SceneComponent.K2_GetComponentLocation` (`self.Mesh`)) (struct) (2.0 2.0 2.0))
        (`ActorComponent.Deactivate` (`self.CharacterMovement`))
        (`KismetSystemLibrary.Delay` 10.0)
        (set `self.Freeze` false)
        (`ActorComponent.Activate` (`self.CharacterMovement`) false)))
    (:`then_3`
      (if (`self.Wind`)
        (`KismetSystemLibrary.Delay` 1.0)
        (set `self.Wind` false)))
    (:`then_4`
      (`|ExecutionSequence`
        (:`then_0`
          (if (`self.Electricity`)
            (`KismetSystemLibrary.Delay` 10.0)
            (set `self.Health` (- (`self.Health`) 5.0))))
        (:`then_1`
          (if (`self.Electricity`)
            (`ActorComponent.Deactivate` (`self.CharacterMovement`))
            (`KismetSystemLibrary.Delay` 10.0)
            (set `self.Electricity` false)
            (`ActorComponent.Activate` (`self.CharacterMovement`) false)))))
    (:`then_5`
      (if (`self.CannonFreeze`)
        (`GameplayStatics.SpawnEmitterAtLocation` "/Game/InfinityBladeEffects/Effects/FX_Monsters/FX_Monster_FrostGiant/ICE/P_ArmBuildUp01.P_ArmBuildUp01" (`SceneComponent.K2_GetComponentLocation` (`self.Mesh`)) (struct) (2.0 2.0 2.0))
        (`ActorComponent.Deactivate` (`self.CharacterMovement`))
        (`KismetSystemLibrary.Delay` 2.0)
        (set `self.Freeze` false)
        (`ActorComponent.Activate` (`self.CharacterMovement`) false)))))

(event `Go to Player`
  ;[1 1 1] ir a enemigo
  (set `CharacterMovementComponent.MaxWalkSpeed` 210.0 (`self.CharacterMovement`))
  (bind _returnvalue (`GameplayStatics.GetActorOfClass` "/Game/Characters/WizzardCharacter/BPCharacter_Wizard.BPCharacter_Wizard_C"))
  (`|AIMoveTo` self (0.0 0.0 0.0) _returnvalue 30.0))

(event `Death`
  ;[1 1 1] Animacion de muerte y destruccion de enemigo
  (`SkeletalMeshComponent.PlayAnimation` (`self.Mesh`) "/Game/NPC/Animations/Sword_And_Shield_Death.Sword_And_Shield_Death" false)
  (`KismetSystemLibrary.Delay` 4.0)
  (bind _asbp_third_person_game_mode (cast `/Game/ThirdPerson/Blueprints/BP_ThirdPersonGameMode` (`GameplayStatics.GetGameMode`)))
  (`/Engine/EditorBlueprintResources/StandardMacros.DecrementInt` (`/Game/ThirdPerson/Blueprints/BP_ThirdPersonGameMode.PaldinAlives` _asbp_third_person_game_mode)
    (:`  `
      (`self.K2_DestroyActor`))))

(event `self.ReceiveAnyDamage`
  (params (Damage :type "Float (single-precision)") (DamageType :type "DamageType Object Reference") (InstigatedBy :type "Controller Object Reference") (DamageCauser :type "Actor Object Reference"))
  ;[1 1 1] Recibir daño
  (bind _output_get (set `self.Health` (- (`self.Health`) Damage)))
  (if (<= _output_get 0.0)
    (set `CharacterMovementComponent.MaxWalkSpeed` 0.0 (`self.CharacterMovement`))
    (`PrimitiveComponent.SetCollisionEnabled` (`self.CapsuleComponent`) "NoCollision")
    (`self.Death`)))

(fn `UserConstructionScript`
  (`parent.UserConstructionScript`))