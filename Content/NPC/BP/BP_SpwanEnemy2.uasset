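; Enemy spawner that periodically spawns goblin AI pawns at its own location in waves.
; After an initial delay on BeginPlay, SpawnEnemy loops by re-calling itself after short delays, incrementing a running count.
; When the count reaches MaxAmount, it pauses, raises the limit by a fixed step and resumes indefinitely.
; Each spawn precedes the limit check, and the count is never decremented or reset.
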(event `self.ReceiveBeginPlay`
  (`KismetSystemLibrary.Delay` 30.0)
  (`self.Spawn Enemy`))

(event `Spawn Enemy`
  (`AIBlueprintHelperLibrary.SpawnAIFromClass` "/Game/NPC/BP/BPC_Goblin.BPC_Goblin_C" null (`self.K2_GetActorLocation`) (struct) false null)
  (if (>= (`self.currentAmount`) (`self.MaxAmount`))
    (`KismetSystemLibrary.Delay` 30.0)
    (set `self.MaxAmount` (+ (`self.MaxAmount`) 10))
    (`self.Spawn Enemy`)
    (else
      (set `self.currentAmount` (+ (`self.currentAmount`) 1))
      (`KismetSystemLibrary.Delay` 2.0)
      (`self.Spawn Enemy`))))

(fn `UserConstructionScript`)