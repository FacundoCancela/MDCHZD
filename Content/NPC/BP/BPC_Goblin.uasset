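; Goblin enemy character that registers in the GameMode's alive count, takes damage and drops a coin on death.
; Tick updates a player-facing health-bar widget and polls status flags with Delays: burn and electricity damage, freezes and electricity halt movement, wind changes the RunSpeed variable.
; Lethal damage plays a death animation before removal.
; A separate door event plays a dance and explodes; both exit paths decrement the count and call EnemysLeft.
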(event `self.ReceiveBeginPlay`
  (set `CharacterMovementComponent.MaxWalkSpeed` (`self.Run Speed`) (`self.CharacterMovement`))
  (bind _asbp_third_person_game_mode (cast `/Game/ThirdPerson/Blueprints/BP_ThirdPersonGameMode` (`GameplayStatics.GetGameMode`)))
  (set `/Game/ThirdPerson/Blueprints/BP_ThirdPersonGameMode.EnemysAlive` (+ (`/Game/ThirdPerson/Blueprints/BP_ThirdPersonGameMode.EnemysAlive` _asbp_third_person_game_mode) 1) _asbp_third_person_game_mode))

(event `self.ReceiveTick`
  (params (DeltaSeconds :type "Float (single-precision)"))
  (`|ExecutionSequence`
    (:`then_0`
      (bind _aswbp_enemy_life (cast `/Game/Widgets/Wenemy/WBP_EnemyLife` (`WidgetComponent.GetUserWidgetObject` (`self.Widget`))))
      (`ProgressBar.SetPercent` (`/Game/Widgets/Wenemy/WBP_EnemyLife.LifeBar` _aswbp_enemy_life) (/ (`self.Health`) 100.0))
      (`SceneComponent.K2_SetWorldRotation` (`self.Widget`) (`KismetMathLibrary.MakeRotator` 0.0 0.0 (.yaw (`KismetMathLibrary.FindLookAtRotation` (`SceneComponent.K2_GetComponentLocation` (`self.Widget`)) (`self.K2_GetActorLocation` (`GameplayStatics.GetPlayerCharacter` 0))))) false false)
      (if (<= (`self.Health`) 0.0)
        (`/Engine/EditorBlueprintResources/StandardMacros.DoOnce` false
          (:`Completed`
            (`PrimitiveComponent.SetSimulatePhysics` (`self.Widget`) true)
            (if (`self.isDead`)
              (`self.K2_DestroyActor`)
              (set `self.isDead` true))))))
    (:`then_1`
      (`|ExecutionSequence`
        (:`then_0`
          (if (`self.Burn`)
            (`KismetSystemLibrary.Delay` 3.0)
            (set `self.Health` (- (`self.Health`) 5.0))))
        (:`then_1`
          (if (`self.Burn`)
            (`KismetSystemLibrary.Delay` 2.0)
            (set `self.Burn` false)))))
    (:`then_2`
      (if (`self.Freeze`)
        (`GameplayStatics.SpawnEmitterAtLocation` "/Game/InfinityBladeEffects/Effects/FX_Monsters/FX_Monster_FrostGiant/ICE/P_ArmBuildUp01.P_ArmBuildUp01" (`SceneComponent.K2_GetComponentLocation` (`self.Mesh`)) (struct) (2.0 2.0 2.0))
        (`ActorComponent.Deactivate` (`self.CharacterMovement`))
        (`KismetSystemLibrary.Delay` 10.0)
        (set `self.Freeze` false)
        (`ActorComponent.Activate` (`self.CharacterMovement`) false)))
    (:`then_3`
      (if (`self.Wind`)
        (set `self.Run Speed` 70.0)
        (`KismetSystemLibrary.Delay` 4.0)
        (set `self.Wind` false)
        (set `self.Run Speed` 350.0)))
    (:`then_4`
      (`|ExecutionSequence`
        (:`then_0`
          (if (`self.Electricity`)
            (`KismetSystemLibrary.Delay` 10.0)
            (set `self.Health` (- (`self.Health`) 5.0))))
        (:`then_1`
          (if (`self.Electricity`)
            (`ActorComponent.Deactivate` (`self.CharacterMovement`))
            (`KismetSystemLibrary.Delay` 10.0)
            (set `self.Electricity` false)
            (`ActorComponent.Activate` (`self.CharacterMovement`) false)))))
    (:`then_5`
      (if (`self.CannonFreeze`)
        (`GameplayStatics.SpawnEmitterAtLocation` "/Game/InfinityBladeEffects/Effects/FX_Monsters/FX_Monster_FrostGiant/ICE/P_ArmBuildUp01.P_ArmBuildUp01" (`SceneComponent.K2_GetComponentLocation` (`self.Mesh`)) (struct) (2.0 2.0 2.0))
        (`ActorComponent.Deactivate` (`self.CharacterMovement`))
        (`KismetSystemLibrary.Delay` 2.0)
        (set `self.Freeze` false)
        (`ActorComponent.Activate` (`self.CharacterMovement`) false)))))

(event `self.ReceiveAnyDamage`
  (params (Damage :type "Float (single-precision)") (DamageType :type "DamageType Object Reference") (InstigatedBy :type "Controller Object Reference") (DamageCauser :type "Actor Object Reference"))
  ;[1 1 1] Evento de Daño y restar vida
  (if (>= (`self.Health`) 0.0)
    (bind _output_get (set `self.Health` (- (`self.Health`) Damage)))
    (if (<= _output_get 0.0)
      (set `CharacterMovementComponent.MaxWalkSpeed` 0.0 (`self.CharacterMovement`))
      (`PrimitiveComponent.SetCollisionEnabled` (`self.CapsuleComponent`) "NoCollision")
      (`self.Death`))))

(event `Death`
  ;[1 1 1] Evento de muerte
  (`SkeletalMeshComponent.PlayAnimation` (`self.Mesh`) "/Game/NPC/Animations/Standing_Death_R.Standing_Death_R" false)
  (`KismetSystemLibrary.Delay` 3.0)
  (`|SpawnActorFromClass` "/Game/Characters/WizzardCharacter/BP_Coin.BP_Coin_C" (`SceneComponent.K2_GetComponentToWorld` (`self.Mesh`)) "Undefined" "OverrideRootScale" null null)
  (`self.DestroyGoblin`))

(event `DestroyGoblin`
  ;[1 1 1] Evento de destrucción de actor
  (bind _asbp_third_person_game_mode (cast `/Game/ThirdPerson/Blueprints/BP_ThirdPersonGameMode` (`GameplayStatics.GetGameMode`)))
  (`/Engine/EditorBlueprintResources/StandardMacros.DecrementInt` (`/Game/ThirdPerson/Blueprints/BP_ThirdPersonGameMode.EnemysAlive` _asbp_third_person_game_mode)
    (:`  `
      (`/Game/ThirdPerson/Blueprints/BP_ThirdPersonGameMode.EnemysLeft` _asbp_third_person_game_mode)
      (set `CharacterMovementComponent.MaxWalkSpeed` 0.0 (`self.CharacterMovement`))
      (`self.K2_DestroyActor`))))

(event `DestroyGoblinInDoor`
  ;[1 1 1] Destruir al Goblin si llega a la puerta
  (bind _asbp_third_person_game_mode (cast `/Game/ThirdPerson/Blueprints/BP_ThirdPersonGameMode` (`GameplayStatics.GetGameMode`)))
  (`/Engine/EditorBlueprintResources/StandardMacros.DecrementInt` (`/Game/ThirdPerson/Blueprints/BP_ThirdPersonGameMode.EnemysAlive` _asbp_third_person_game_mode)
    (:`  `
      (`/Game/ThirdPerson/Blueprints/BP_ThirdPersonGameMode.EnemysLeft` _asbp_third_person_game_mode)
      (set `CharacterMovementComponent.MaxWalkSpeed` 0.0 (`self.CharacterMovement`))
      (`PrimitiveComponent.SetCollisionEnabled` (`self.CapsuleComponent`) "NoCollision")
      (`SkeletalMeshComponent.PlayAnimation` (`self.Mesh`) "/Game/NPC/Animations/Breakdance_Footwork_To_Idle.Breakdance_Footwork_To_Idle" false)
      (`KismetSystemLibrary.Delay` 6.0)
      (`GameplayStatics.SpawnEmitterAtLocation` "/Game/StarterContent/Particles/P_Explosion.P_Explosion" (`SceneComponent.K2_GetComponentLocation` (`self.Mesh`)))
      (`self.K2_DestroyActor`))))

(fn `UserConstructionScript`)